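; Parent Blueprint for employee characters that can hold a task and offer it through an interact prompt.
; Givetask flags the task, prints a debug message and shows the text prompt immediately, regardless of overlap.
; Box overlap enables the prompt and interaction only while a task is held, and leaving hides both.
; GetTask calls SayTask, which has no body here, when interaction is allowed and a task exists.
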(event OnComponentBeginOverlap(Box)
  (params (OverlappedComponent :type Primitive%20Component%20Object%20Reference) (OtherActor :type Actor%20Object%20Reference) (OtherComp :type Primitive%20Component%20Object%20Reference) (OtherBodyIndex :type Integer) (bFromSweep :type Boolean) (SweepResult :type Hit%20Result%20Structure%20%28by%20ref%29))
  ;[0.15 0.15 0.15 0.5] Shows interact prompt when there's a task
  (if (Variables|Default|GethasTask)
    (Rendering|SetVisibility (Variables|Default|GetTextRender) true false)
    (Variables|Default|SetcanInteract true)))

(event OnComponentEndOverlap(Box)
  (params (OverlappedComponent :type Primitive%20Component%20Object%20Reference) (OtherActor :type Actor%20Object%20Reference) (OtherComp :type Primitive%20Component%20Object%20Reference) (OtherBodyIndex :type Integer))
  ;[0.15 0.15 0.15 0.5] Shows interact prompt when there's a task
  (Rendering|SetVisibility (Variables|Default|GetTextRender) false false)
  (Variables|Default|SetcanInteract false))

(event Custom|Give%20task
  (Variables|Default|SethasTask true)
  (Development|PrintString "task given")
  (Rendering|SetVisibility (Variables|Default|GetTextRender) true false))

(event EventBeginPlay)

(event EventGetTask
  (if (and (Variables|Default|GetcanInteract) (Variables|Default|GethasTask))
    (CallFunction|SayTask)))

(fn ConstructionScript)